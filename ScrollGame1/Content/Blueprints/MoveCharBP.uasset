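; Player character Blueprint with camera-relative movement, an energy-limited dash, a sword slash attack and a SampleUI widget added at BeginPlay.
; Energy refills on Tick and drains while Dash is held, gating full-speed forward/back input, while strafing dashes regardless of Energy.
; Left click plays the slash montage, locked by IsAttacking until the animation-end event.
; Attack collision events toggle the Capsule hitbox, whose overlaps only print the other actor's name.
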(event OnComponentBeginOverlap(Capsule)
  (params (OverlappedComponent :type Primitive%20Component%20Object%20Reference) (OtherActor :type Actor%20Object%20Reference) (OtherComp :type Primitive%20Component%20Object%20Reference) (OtherBodyIndex :type Integer) (bFromSweep :type Boolean) (SweepResult :type Hit%20Result%20Structure%20%28by%20ref%29))
  (if (not (== OtherActor self))
    (Development|PrintString (Utilities|GetDisplayName OtherActor))))

(event Custom|OnAnimEnd_Attack
  (Variables|Default|SetIsAttacking false))

(event Custom|OnCollStart_Attack
  (Collision|SetCollisionEnabled (Variables|Default|GetCapsule) "QueryAndPhysics"))

(event Custom|OnCollEnd_Attack
  (Collision|SetCollisionEnabled (Variables|Default|GetCapsule) "NoCollision"))

(event EventBeginPlay
  (bind _returnvalue (UserInterface|CreateWidget "/Game/Blueprints/SampleUI.SampleUI_C"))
  (bind _output_get (Variables|Default|SetNewVar_0 _returnvalue))
  (UserInterface|Viewport|AddtoViewport _output_get 0))

(event EventTick
  (params (DeltaSeconds :type Float%20%28single-precision%29))
  (if (< (Variables|Default|GetEnergy) 1.0)
    (Variables|Default|SetEnergy (+ (Variables|Default|GetEnergy) 0.01))))

(event Input|ActionEvents|InputActionDash
  (params (Key :type Key%20Structure))
  (:Pressed
    (Variables|Default|SetIsDash true))
  (:Released
    (Variables|Default|SetIsDash false)))

(event Input|AxisEvents|InputAxisTurn
  (params (AxisValue :type Float%20%28single-precision%29))
  (Pawn|Input|AddControllerYawInput AxisValue))

(event Input|AxisEvents|InputAxisLookUp
  (params (AxisValue :type Float%20%28single-precision%29))
  (Pawn|Input|AddControllerPitchInput AxisValue))

(event Input|AxisEvents|InputAxisLeftRight
  (params (AxisValue :type Float%20%28single-precision%29))
  (bind _returnvalue (Pawn|GetControlRotation :!class /Script/Engine.Pawn))
  (bind _yaw (Math|Rotator|BreakRotator _returnvalue))
  (bind _returnvalue_2 (Math|Rotator|MakeRotator 0.0 0.0 _yaw))
  (bind _returnvalue_3 (Math|Vector|GetRightVector _returnvalue_2))
  (if (Variables|Default|GetIsDash)
    (Pawn|Input|AddMovementInput _returnvalue_3 (* AxisValue 1.0) false)
    (else
      (Pawn|Input|AddMovementInput _returnvalue_3 (* AxisValue 0.5) false))))

(event Input|AxisEvents|InputAxisForwardBackward
  (params (AxisValue :type Float%20%28single-precision%29))
  (bind _returnvalue (Pawn|GetControlRotation :!class /Script/Engine.Pawn))
  (bind _yaw (Math|Rotator|BreakRotator _returnvalue))
  (bind _returnvalue_2 (Math|Rotator|MakeRotator 0.0 0.0 _yaw))
  (bind _returnvalue_3 (Math|Vector|GetForwardVector _returnvalue_2))
  (if (Variables|Default|GetIsDash)
    (if (>= (Variables|Default|GetEnergy) 0.0)
      (Variables|Default|SetEnergy (- (Variables|Default|GetEnergy) 0.02))
      (Pawn|Input|AddMovementInput _returnvalue_3 (* AxisValue 1.0) false)
      (else
        (Pawn|Input|AddMovementInput _returnvalue_3 (* AxisValue 0.5) false :!label _label)))
    (else
      (goto _label))))

(event Input|MouseEvents|LeftMouseButton
  (params (Key :type Key%20Structure))
  (:Pressed
    (if (not (Variables|Default|GetIsAttacking))
      (Variables|Default|SetIsAttacking true)
      (Animation|PlayAnimMontage "/Game/Mesh/Paladin/Animations/sword_and_shield_slash_Montage.sword_and_shield_slash_Montage" 1.0 "None"))))

(fn ConstructionScript)