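; MoveActorBP is an actor Blueprint that the player moves horizontally with input axes.
; BeginPlay enables input from player controller 0 so the actor receives the ForwardBackward and LeftRight axes.
; Each axis event adds a fixed offset scaled by the axis value along world X or inverted world Y.
; Movement sets the location directly without sweep or delta time, so it ignores collision and depends on frame rate.
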(event EventBeginPlay
  (Input|EnableInput (Game|GetPlayerController 0)))

(event Input|AxisEvents|InputAxisForwardBackward
  (params (AxisValue :type Float%20%28single-precision%29))
  (Transformation|SetActorLocation (+ (* (Math|Conversions|ToVector(Float) AxisValue) (Math|Vector|MakeVector 5.0 0.0 0.0)) (Transformation|GetActorLocation)) false false))

(event Input|AxisEvents|InputAxisLeftRight
  (params (AxisValue :type Float%20%28single-precision%29))
  (Transformation|SetActorLocation (+ (* (Math|Conversions|ToVector(Float) AxisValue) (Math|Vector|MakeVector 0.0 -5.0 0.0)) (Transformation|GetActorLocation)) false false))

(fn ConstructionScript)